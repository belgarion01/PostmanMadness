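; BP_Papers is a physics-driven papers projectile that can be posted to targets in the game.
; On BeginPlay it launches its static mesh at a stored velocity.
; A Collision overlap notifies any actor implementing IPostable through OnPosted, passing itself.
; The first mesh hit zeroes the velocity and enables gravity, so it flies until impact and then drops, with a flag preventing repeats.
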(event `self.ReceiveBeginPlay`
  (`PrimitiveComponent.SetPhysicsLinearVelocity` (`self.StaticMesh`) (`self.Velocity`) false "None")
  (set `self.Enabled` true))

(event `self.Collision.OnComponentBeginOverlap`
  (params (OverlappedComponent :type "PrimitiveComponent Object Reference") (OtherActor :type "Actor Object Reference") (OtherComp :type "PrimitiveComponent Object Reference") (OtherBodyIndex :type Integer) (bFromSweep :type Boolean) (SweepResult :type "HitResult Structure (by ref)"))
  (bind _asipostable (cast `/Game/PostmanMadness/Blueprints/IPostable` OtherActor))
  (`/Game/PostmanMadness/Blueprints/IPostable.OnPosted` _asipostable self))

(event `self.StaticMesh.OnComponentHit`
  (params (HitComponent :type "PrimitiveComponent Object Reference") (OtherActor :type "Actor Object Reference") (OtherComp :type "PrimitiveComponent Object Reference") (NormalImpulse :type "Vector Structure") (Hit :type "HitResult Structure (by ref)"))
  (bind _staticmesh (`self.StaticMesh`))
  (if (`self.Enabled`)
    (`PrimitiveComponent.SetPhysicsLinearVelocity` _staticmesh (0.0 0.0 0.0) false "None")
    (`PrimitiveComponent.SetEnableGravity` _staticmesh true)
    (set `self.Enabled` false)))

(fn `UserConstructionScript`)