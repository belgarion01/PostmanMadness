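; Player controller for the postman character that lets the player throw newspapers toward the mouse cursor.
; It adds the default Enhanced Input mapping context on BeginPlay and caches the possessed pawn as a BP_Postman.
; When the throw action completes, it traces under the cursor on the Visibility channel and, on a hit, passes the normalized 2D direction from the postman to that point into ThrowNewspaper.
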(event `self.ReceiveBeginPlay`
  (bind _returnvalue (subsystem `EnhancedInputLocalPlayerSubsystem`))
  (`/Engine/EditorBlueprintResources/StandardMacros.IsValid` _returnvalue
    (:`Is Valid`
      (`EnhancedInputSubsystemInterface.AddMappingContext` _returnvalue "/Game/PostmanMadness/Blueprints/Inputs/IMC_Default.IMC_Default" 0 (struct)))))

(event `self.ReceivePossess`
  (params (PossessedPawn :type "Pawn Object Reference"))
  (bind _asbp_postman (cast `/Game/PostmanMadness/Blueprints/Characters/BP_Postman` PossessedPawn))
  (set `self.Postman` _asbp_postman))

(event `EnhancedInput|/Game/PostmanMadness/Blueprints/Inputs/IA_Throw`
  (params (ActionValue :type Boolean) (ElapsedSeconds :type "Float (double-precision)") (TriggeredSeconds :type "Float (double-precision)") (InputAction :type "InputAction Object Reference" :default "/Game/PostmanMadness/Blueprints/Inputs/IA_Throw.IA_Throw"))
  (bind (_hit _location) (`self.GetLocationUnderCursor`))
  (:`Completed`
    (if _hit
      (bind _postman (`self.Postman`)
        (:`then`
          (`/Game/PostmanMadness/Blueprints/Characters/BP_Postman.ThrowNewspaper` _postman (`KismetMathLibrary.Normal2D` (`KismetMathLibrary.Conv_VectorToVector2D` (- _location (`self.K2_GetActorLocation` (`self.Postman`)))))))
        (:`else`)))))

(fn `GetLocationUnderCursor`
  (returns (Hit :type Boolean) (Location :type "Vector Structure"))
  (bind (_bblockinghit _binitialoverlap _time _distance _location) (`GameplayStatics.BreakHitResult` (`self.GetHitResultUnderCursorByChannel` "TraceTypeQuery1")))
  (return _bblockinghit _location))

(fn `UserConstructionScript`)