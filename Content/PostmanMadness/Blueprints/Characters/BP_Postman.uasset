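; BP_Postman is the postman character, which moves relative to the camera and throws newspapers.
; Each Tick feeds the horizontal and vertical input axes, scaled by Acceleration, into AddMovementInput along the camera's flattened right and forward vectors.
; ThrowNewspaper spawns BP_Papers at the actor, passing itself as owner and a fixed-speed velocity along the given 2D direction.
; A custom velocity model in ComputeVelocity and an acceleration interpolation are present but never run.
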(event `self.ReceiveTick`
  (params (DeltaSeconds :type "Float (single-precision)"))
  (bind _camera (`self.Camera`))
  (set `self.DeltaTime` DeltaSeconds)
  (`|ExecutionSequence`
    (:`then_0`
      (`self.AddMovementInput` (`KismetMathLibrary.MakeVector` (.x (`SceneComponent.GetRightVector` _camera)) (.y (`SceneComponent.GetRightVector` _camera))) (* (`|GetInputActionValue`) (`self.Acceleration`)))
      (`self.AddMovementInput` (`KismetMathLibrary.MakeVector` (.x (`SceneComponent.GetForwardVector` _camera)) (.y (`SceneComponent.GetForwardVector` _camera))) (* (`|GetInputActionValue`) (`self.Acceleration`))))))

(event `ThrowNewspaper`
  (params (Direction :type "Vector2D Structure"))
  (`|SpawnActorFromClass` "/Game/PostmanMadness/Blueprints/BP_Papers.BP_Papers_C" (`KismetMathLibrary.MakeTransform` (`self.K2_GetActorLocation`) (`KismetMathLibrary.Conv_VectorToRotator` (`KismetMathLibrary.Conv_Vector2DToVector` Direction))) "Undefined" "MultiplyWithRoot" null self (* (`KismetMathLibrary.Conv_Vector2DToVector` Direction) 3000.0) null))

(fn `ComputeVelocity`
  (bind _returnvalue (`|GetInputActionValue`))
  (bind _camera (`self.Camera`))
  (if (or (!= (`|GetInputActionValue`) 0.0) (!= (`|GetInputActionValue`) 0.0))
    (set `self.Velocity` (`KismetMathLibrary.ClampVectorSize` (+ (`self.Velocity`) (* (`KismetMathLibrary.Normal` (+ (* (`KismetMathLibrary.MakeVector` (.x (`SceneComponent.GetRightVector` _camera)) (.y (`SceneComponent.GetRightVector` _camera))) (`KismetMathLibrary.MakeVector` _returnvalue _returnvalue)) (* (`KismetMathLibrary.MakeVector` (.x (`SceneComponent.GetForwardVector` _camera)) (.y (`SceneComponent.GetForwardVector` _camera))) (`|GetInputActionValue`)))) (`self.Acceleration`) (`self.DeltaTime`))) 0.0 (`self.MaxSpeed`)))))

(fn `UserConstructionScript`)