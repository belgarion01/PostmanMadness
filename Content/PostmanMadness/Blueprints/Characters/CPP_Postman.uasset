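; Postman player character that drives forward with vehicle-like acceleration, braking and steering, and throws newspapers.
; Each tick, vertical input raises or brakes a clamped Speed that sets max walk speed, while forward movement input is applied whenever Speed is positive.
; Horizontal input yaws the actor, and current speed is printed for debugging.
; ThrowNewspaper spawns BP_Papers at the actor with a fixed-speed velocity along the given 2D direction.
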(event `ThrowNewspaper`
  (params (Direction :type "Vector2D Structure"))
  ;[1 1 1] Launching Papers
  (`|SpawnActorFromClass` "/Game/PostmanMadness/Blueprints/BP_Papers.BP_Papers_C" (`KismetMathLibrary.MakeTransform` (`self.K2_GetActorLocation`) (`KismetMathLibrary.Conv_VectorToRotator` (`KismetMathLibrary.Conv_Vector2DToVector` Direction))) "Undefined" "MultiplyWithRoot" null self (* (`KismetMathLibrary.Conv_Vector2DToVector` Direction) 3000.0) null))

(event `self.ReceiveTick`
  (params (DeltaSeconds :type "Float (single-precision)"))
  (set `self.DeltaTime` DeltaSeconds)
  (`|ExecutionSequence`
    (:`then_0`
      ;[1 1 1] Set controller settings
      (set `CharacterMovementComponent.MaxWalkSpeed` (`self.Speed`) (`self.CharacterMovement`))
      ;[1 1 1] Is Breaking
      (set `self.IsBreaking` (< (`|GetInputActionValue`) 0.0)))
    (:`then_1`
      (if (`self.IsBreaking`)
        ;[1 1 1] Breaking
        (set `self.Speed` (`KismetMathLibrary.FMax` (- (`self.Speed`) (* (`self.BreakingForce`) (`self.DeltaTime`)))))
        (else
          ;[1 1 1] Accelerating
          (set `self.Speed` (`KismetMathLibrary.FClamp` (+ (`self.Speed`) (* (`|GetInputActionValue`) (`self.Acceleration`) (`self.DeltaTime`))) 0.0 (`self.MaxSpeed`))))))
    (:`then_2`
      ;[1 1 1] Apply Movement
      (`self.AddMovementInput` (`self.GetActorForwardVector`) (`KismetMathLibrary.SelectFloat` 1.0 0.0 (> (`self.Speed`) 0.0)) true)
      (`self.K2_AddActorWorldRotation` (`KismetMathLibrary.MakeRotator` 0.0 0.0 (* (`|GetInputActionValue`) (`self.RotationSpeed`) (`self.DeltaTime`)))))
    (:`then_3`
      ;[1 1 1] Print values
      (`/Game/PostmanMadness/Blueprints/Utilities/BPFL_Utilities.PrintTickText` (`|FormatText` "Speed: {Speed}" (`self.Speed`))))))

(fn `UserConstructionScript`)